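; Brazier actor that starts dark and lights once when an AlexandriaCharacter with InnerRadiance enters its DistCheck trigger, which is then destroyed.
; Tick runs a LitState machine that scales the fire particles and light color, captured at construction, along float curves over EclipseTime.
; EclipseStart switches to the eclipse curve and deactivates the particles when the timer ends.
; EclipseEnd is a stub returning false.
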(event `self.ReceiveBeginPlay`
  (`LightComponent.SetLightColor` :`self` (`self.FireLight`)))

(event `self.ReceiveTick`
  (params (DeltaSeconds :type "Float (single-precision)"))
  (bind _temptime (`self.TempTime`))
  (bind _litstate (`self.LitState`))
  (bind _returnvalue (/ _temptime (`self.EclipseTime`)))
  (bind _returnvalue_2 (`KismetMathLibrary.SelectFloat` (`CurveFloat.GetFloatValue` (`self.LightOnCurve`) _returnvalue) (`CurveFloat.GetFloatValue` (`self.EclipseStartCurve`) _returnvalue) (== _litstate 1)))
  (switch `int` _litstate :!label _label
    (:`1`
      (`ActorComponent.Activate` (`self.ParticleSystem`) false))
    (:`2`
      _))
  (`SceneComponent.SetRelativeScale3D` (`self.ParticleSystem`) (* (`self.ParticleScale`) _returnvalue_2))
  (`LightComponent.SetLightColor` (`self.FireLight`) (* (`self.FireLightColor`) _returnvalue_2) true)
  (bind _output_get (set `self.TempTime` (+ _temptime DeltaSeconds)))
  (if (>= _output_get (`self.EclipseTime`))
    (switch `int` (`self.LitState`)
      (:`1`
        _)
      (:`2`
        (`ActorComponent.Deactivate` (`self.ParticleSystem`))))
    (set `self.TempTime` 0.0)
    (set `self.LitState` 0)))

(event `self.DistCheck.OnComponentBeginOverlap`
  (params (OverlappedComponent :type "PrimitiveComponent Object Reference") (OtherActor :type "Actor Object Reference") (OtherComp :type "PrimitiveComponent Object Reference") (OtherBodyIndex :type Integer) (bFromSweep :type Boolean) (SweepResult :type "HitResult Structure (by ref)"))
  (bind _asalexandria_character (cast `/Game/Alexandria/Character/AlexandriaCharacter` OtherActor))
  (if (`AlexandriaCharacter.bInnerRadiance` _asalexandria_character)
    (set `self.LitState` 1)
    (set `self.TempTime` 0.0)
    (`ActorComponent.K2_DestroyComponent` (`self.DistCheck`))
    (goto _label)))

(event `self.ParticleSystem.OnComponentActivated`
  (params (Component :type "ActorComponent Object Reference") (bReset :type Boolean)))

(fn `EclipseEnd`
  (returns (Eclipse :type Boolean))
  (return false))

(fn `EclipseStart`
  (returns (Eclipse :type Boolean))
  (set `self.TempTime` 0.0)
  (bind _output_get (set `self.LitState` 2))
  (return (== _output_get 2)))

(fn `UserConstructionScript`
  (set `self.FireLightColor` (`LightComponentBase.GetLightColor` (`self.FireLight`)))
  (set `self.ParticleScale` (.scale (`SceneComponent.GetRelativeTransform` (`self.ParticleSystem`)))))